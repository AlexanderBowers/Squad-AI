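; BP_FirePoint is a squad command point that toggles the priority assignment of one squad member to it.
; CheckAssignedMember resets and clears a valid assigned member, or otherwise gets an available one from SquadPlayerController for the given CommandPoint and flags it as priority.
; The Hit event only prints debug text, comparing the trace start to the controller's location when a SquadPlayerController or Commando hits it.
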(event EventBeginPlay)

(event Collision|EventActorBeginOverlap
  (params (OtherActor :type Actor%20Object%20Reference)))

(event EventTick
  (params (DeltaSeconds :type Float%20%28single-precision%29)))

(event Collision|EventHit
  (params (MyComp :type Primitive%20Component%20Object%20Reference) (Other :type Actor%20Object%20Reference) (OtherComp :type Primitive%20Component%20Object%20Reference) (bSelfMoved :type Boolean) (HitLocation :type Vector :default "0, 0, 0") (HitNormal :type Vector :default "0, 0, 0") (NormalImpulse :type Vector :default "0, 0, 0") (Hit :type Hit%20Result%20Structure%20%28by%20ref%29))
  (bind _tracestart (Collision|BreakHitResult Hit))
  (bind _assquad_player_controller (Utilities|Casting|CastToSquadPlayerController Other)
    (:then
      (if (Math|Vector|Equal(Vector) _tracestart (Transformation|GetActorLocation _assquad_player_controller) 0.0001)
        (Development|PrintText "Location Matched")
        (else
          (Development|PrintText "Location Failed"))))
    (:CastFailed
      (Development|PrintText "Cast Failed")
      (Utilities|Casting|CastToCommando Other
        (:then
          (if (Math|Vector|Equal(Vector) _tracestart (Transformation|GetActorLocation (Game|GetPlayerController 0)) 0.0001)
            (Development|PrintText "Location Matched")
            (else
              (Development|PrintText "Location Failed"))))
        (:CastFailed
          (Development|PrintText "Uh Oh"))))))

(event EventCheckAssignedMember
  (params (CommandPoint :type Command%20Pointy%20Structure))
  (Utilities|IsValid (Variables|Default|GetAssignedSquadMember)
    (:Is%20Valid
      (Development|PrintText "IsValid")
      (Class|SquadAIController|ResetPriorityCommand (Variables|Default|GetAssignedSquadMember))
      (Variables|Default|SetAssignedSquadMember 0)
      (Development|PrintText "Should now be invalid"))
    (:Is%20Not%20Valid
      (bind _assquad_player_controller (Utilities|Casting|CastToSquadPlayerController (Game|GetPlayerController 0)))
      (bind _returnvalue (Class|SquadPlayerController|GetAvailableMember _assquad_player_controller CommandPoint))
      (Variables|/Script/Squad.SquadAIController|SetbHasPriority _returnvalue true)
      (Variables|Default|SetAssignedSquadMember _returnvalue)
      (Development|PrintText "It worked!!!"))))

(fn ConstructionScript)