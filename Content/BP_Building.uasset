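; BP_Building is a building actor that uses overlap events to tell squad controllers when a Commando enters or leaves it.
; AI-controlled commandos get their SquadAIController's IsIndoors flag set or cleared, plus a reference to the building on entry.
; For any other commando, player 0's SquadPlayerController calls GetRooms with this building on entry and FormUpCommand on exit.
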(event EventBeginPlay)

(event Collision|EventActorBeginOverlap
  (params (OtherActor :type Actor%20Object%20Reference))
  (bind _self self)
  (bind _ascommando (Utilities|Casting|CastToCommando OtherActor))
  (bind _assquad_aicontroller (Utilities|Casting|CastToSquadAIController (AI|GetAIController _ascommando))
    (:then
      (Variables|/Script/Squad.SquadAIController|SetbIsIndoors _assquad_aicontroller true)
      (Variables|/Script/Squad.SquadAIController|SetBuilding _assquad_aicontroller _self))
    (:CastFailed
      (bind _assquad_player_controller (Utilities|Casting|CastToSquadPlayerController (Game|GetPlayerController 0)))
      (Class|SquadPlayerController|GetRooms _assquad_player_controller _self))))

(event EventTick
  (params (DeltaSeconds :type Float%20%28single-precision%29)))

(event Collision|EventActorEndOverlap
  (params (OtherActor :type Actor%20Object%20Reference))
  (bind _ascommando (Utilities|Casting|CastToCommando OtherActor))
  (bind _assquad_aicontroller (Utilities|Casting|CastToSquadAIController (AI|GetAIController _ascommando))
    (:then
      (Variables|/Script/Squad.SquadAIController|SetbIsIndoors _assquad_aicontroller false))
    (:CastFailed
      (bind _assquad_player_controller (Utilities|Casting|CastToSquadPlayerController (Game|GetPlayerController 0)))
      (Class|SquadPlayerController|FormUpCommand _assquad_player_controller))))

(fn ConstructionScript)