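; Squad AI controller that feeds perceived targets into its Blackboard.
; BeginPlay seeds the Blackboard with a starting Health value and clears IsDead.
; AI Perception updates pass the actor through IsEnemyTeam, which only casts to BP_AI_Character without comparing teams, then store it as TargetActor, with no sensed-or-lost check.
; SetTargetActor_0 is an uncalled duplicate of SetTargetActor.
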(event OnTargetPerceptionUpdated(AIPerception)
  (params (Actor :type Actor%20Object%20Reference) (Stimulus :type AI%20Stimulus%20Structure))
  (bind (_isenemyteam _enemyai) (CallFunction|IsEnemyTeam? Actor))
  (if _isenemyteam
    (CallFunction|SetTargetActor _enemyai)))

(event EventBeginPlay
  (bind _self self)
  (bind _returnvalue (AI|GetBlackboard _self))
  (AI|Components|Blackboard|SetValueasFloat _returnvalue (Utilities|Name|MakeLiteralName "Health") 1e+04)
  (AI|Components|Blackboard|SetValueasBool _returnvalue (Utilities|Name|MakeLiteralName "IsDead") false))

(event EventTick
  (params (DeltaSeconds :type Float%20%28single-precision%29)))

(fn ConstructionScript)

(fn SetTargetActor
  (params (TheTargetActor :type Actor%20Object%20Reference))
  (AI|Components|Blackboard|SetValueasObject (AI|GetBlackboard self) (Utilities|Name|MakeLiteralName "TargetActor") TheTargetActor)
  (return TheTargetActor))

(fn IsEnemyTeam?
  (params (Enemy :type Object%20Object%20Reference))
  (bind _asbp_ai_character (Utilities|Casting|CastToBP_AI_Character Enemy))
  (return true _asbp_ai_character))

(fn SetTargetActor0
  (params (TheTargetActor :type Actor%20Object%20Reference))
  (AI|Components|Blackboard|SetValueasObject (AI|GetBlackboard self) (Utilities|Name|MakeLiteralName "TargetActor") TheTargetActor)
  (return TheTargetActor))