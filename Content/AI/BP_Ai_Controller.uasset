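; AI controller that runs the BT_Basic behavior tree and targets Commando actors detected through AI perception.
; On BeginPlay it starts the tree and seeds the blackboard's Health and IsDead keys.
; Perception updates write any actor that casts to Commando into TargetActor; this cast is the only enemy-team check, and the target is never cleared.
; Helper functions read the target back and report whether it is valid.
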(event OnTargetPerceptionUpdated(AIPerception)
  (params (Actor :type Actor%20Object%20Reference) (Stimulus :type AI%20Stimulus%20Structure))
  (bind (_isenemyteam _enemyai) (CallFunction|IsEnemyTeam? Actor))
  (if _isenemyteam
    (CallFunction|SetTargetActor _enemyai)))

(event EventBeginPlay
  (bind _self self)
  (bind _returnvalue (AI|GetBlackboard _self))
  (AI|RunBehaviorTree "/Game/AI/BT_Basic.BT_Basic")
  (AI|Components|Blackboard|SetValueasFloat _returnvalue (Utilities|Name|MakeLiteralName "Health") 1e+02)
  (AI|Components|Blackboard|SetValueasBool _returnvalue (Utilities|Name|MakeLiteralName "IsDead") false))

(event EventTick
  (params (DeltaSeconds :type Float%20%28single-precision%29)))

(fn ConstructionScript)

(fn GetTargetActor
  (bind _ascommando (Utilities|Casting|CastToCommando (AI|Components|Blackboard|GetValueasObject (AI|GetBlackboard self) (Utilities|Name|MakeLiteralName "TargetActor"))))
  (return _ascommando))

(fn IsEnemyTeam?
  (params (Enemy :type Object%20Object%20Reference))
  (bind _ascommando (Utilities|Casting|CastToCommando Enemy))
  (return true _ascommando))

(fn SetTargetActor
  (params (TheTargetActor :type Commando%20Object%20Reference))
  (AI|Components|Blackboard|SetValueasObject (AI|GetBlackboard self) (Utilities|Name|MakeLiteralName "TargetActor") TheTargetActor)
  (return TheTargetActor))

(fn IsTargetActorSet
  (bind _returnvalue (Utilities|Name|MakeLiteralName "TargetActor"))
  (bind _self self)
  (bind _returnvalue_2 (AI|GetBlackboard _self))
  (bind _returnvalue_3 (AI|Components|Blackboard|GetValueasObject _returnvalue_2 _returnvalue))
  (bind _ascommando (Utilities|Casting|CastToCommando _returnvalue_3))
  (return _ascommando (Utilities|IsValid _returnvalue_3)))