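; AI controller for squad members that runs the BT_Commando behavior tree and seeds its blackboard with a very large Health and a cleared IsDead flag.
; On perception updates, it casts the sensed actor to BP_AI_Character and treats it as an enemy when their blackboard Team strings differ.
; Detected enemies are passed to SetTargetActor, which is an empty stub, so no target is stored.
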(event OnTargetPerceptionUpdated(AIPerception)
  (params (Actor :type Actor%20Object%20Reference) (Stimulus :type AI%20Stimulus%20Structure))
  (bind (_isenemyteam _enemyai) (CallFunction|IsEnemyTeam? Actor))
  (if _isenemyteam
    (CallFunction|SetTargetActor _enemyai)))

(event EventBeginPlay
  (bind _self self)
  (bind _returnvalue (AI|GetBlackboard _self))
  (AI|RunBehaviorTree "/Game/AI/BT_Commando.BT_Commando")
  (AI|Components|Blackboard|SetValueasFloat _returnvalue (Utilities|Name|MakeLiteralName "Health") 1e+08)
  (AI|Components|Blackboard|SetValueasBool _returnvalue (Utilities|Name|MakeLiteralName "IsDead") false))

(event EventTick
  (params (DeltaSeconds :type Float%20%28single-precision%29)))

(fn ConstructionScript)

(fn SetTargetActor
  (params (TheTargetActor :type BP%20AI%20Character%20Object%20Reference))
  (return 0))

(fn IsEnemyTeam?
  (params (Enemy :type Object%20Object%20Reference))
  (bind _asbp_ai_character (Utilities|Casting|CastToBP_AI_Character Enemy))
  (return (Utilities|Enum|NotEqual(Enum) (Class|BlackboardComponent|GetValueasString (AI|GetBlackboard self) (Utilities|Name|MakeLiteralName "Team")) (Class|BlackboardComponent|GetValueasString (AI|GetBlackboard _asbp_ai_character) (Utilities|Name|MakeLiteralName "Team"))) _asbp_ai_character))