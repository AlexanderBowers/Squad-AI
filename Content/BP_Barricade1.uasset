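; BP_Barricade1 is a squad-commandable barricade where an assigned commando plants a bomb.
; CheckAssignedMember requests an available member from the SquadPlayerController for a command at BombLocation, gives it priority and starts a three-second timer.
; When that member's Commando pawn overlaps the barricade, it spawns BP_Bomb at BombLocation.
; SetBombTimer is an empty stub, and the assignment reset includes unconnected calls.
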(event Custom|SetBombTimer)

(event EventBeginPlay)

(event Collision|EventActorBeginOverlap
  (params (OtherActor :type Actor%20Object%20Reference))
  (bind _ascommando (Utilities|Casting|CastToCommando OtherActor)
    (:then
      (if (== (Pawn|GetControlledPawn (Variables|Default|GetAssignedSquadMember)) _ascommando)
        (Game|SpawnActorfromClass "/Game/BP_Bomb.BP_Bomb_C" (Transformation|GetWorldTransform (Variables|Default|GetBombLocation)) "Undefined" 0 0)
        (CallFunction|SetBombTimer)
        (else
          (Development|PrintText "Failed :("))))
    (:CastFailed
      (Development|PrintText "Cast failed!!"))))

(event EventTick
  (params (DeltaSeconds :type Float%20%28single-precision%29)))

(event EventResetAssignedMember
  (Utilities|IsValid (Variables|Default|GetAssignedSquadMember)
    (:Is%20Valid
      (Variables|Default|SetAssignedSquadMember 0))
    (:Is%20Not%20Valid
      (Development|PrintString "Reset Called but not valid."))))

(event EventCheckAssignedMember
  (params (CommandPoint :type Command%20Pointy%20Structure))
  (bind (_location _type _owneractor) (Utilities|Struct|BreakCommandPointy CommandPoint))
  (Utilities|IsValid (Variables|Default|GetAssignedSquadMember)
    (:Is%20Not%20Valid
      (bind _assquad_player_controller (Utilities|Casting|CastToSquadPlayerController (Game|GetPlayerController 0)))
      (bind _returnvalue (Class|SquadPlayerController|GetAvailableMember _assquad_player_controller (Utilities|Struct|MakeCommandPointy (Transformation|GetWorldLocation (Variables|Default|GetBombLocation)) _type _owneractor)))
      (Variables|/Script/Squad.SquadAIController|SetAssignedPosition _returnvalue self)
      (Variables|/Script/Squad.SquadAIController|SetbHasPriority _returnvalue true)
      (Variables|Default|SetAssignedSquadMember _returnvalue)
      (Utilities|Time|SetTimerbyEvent (EventDispatchers|CreateEvent :!event Custom|SetBombTimer) 3.0))))

(fn ConstructionScript)